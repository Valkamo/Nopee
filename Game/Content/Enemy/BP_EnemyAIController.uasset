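; BP_EnemyAIController is an enemy AI controller that chases and attacks the player.
; SetTarget stores the player reference, enables movement and starts a looping timer that calls FollowPlayer.
; Each tick of that timer moves the pawn toward the player with MoveToActor, then casts it to BP_EnemyCharacter and calls TryShootPlayer, leaving a debug print in place.
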(event `SetTarget`
  (params (NewParam :type "/Game/Variant_Platforming/Blueprints/BP_PlayerCharacter Object Reference"))
  (set `self.PlayerRef` NewParam)
  (set `self.CanMove` true)
  (`KismetSystemLibrary.K2_SetTimer` null "FollowPlayer" 0.3 true))

(fn `FollowPlayer`
  (bind _playerref (`self.PlayerRef`))
  (if (`self.CanMove`)
    (`/Engine/EditorBlueprintResources/StandardMacros.IsValid` _playerref
      (:`Is Valid`
        (`self.MoveToActor` _playerref 100.0 true true true "/Script/AIModule.NavFilter_AIControllerDefault")
        (`KismetSystemLibrary.PrintString` "CASTING")
        (bind _asbp_enemy_character (cast `/Game/Enemy/BP_EnemyCharacter` (`self.K2_GetPawn`)))
        (`/Game/Enemy/BP_EnemyCharacter.TryShootPlayer` _asbp_enemy_character)))))

(fn `UserConstructionScript`)