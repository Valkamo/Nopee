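; Enemy character that spots the player, shoots with a hitscan gun and ragdolls on death.
; AI perception updates store the player and pass it as target to BP_EnemyAIController.
; TryShootPlayer checks range and facing, then line-traces from the gun barrel with accuracy-based random spread, damaging whatever it hits; only hits start the fire-rate cooldown.
; Incoming damage drains Health until death enables mesh physics and destroys the actor after a short delay.
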(event `self.ReceiveBeginPlay`
  ; AI perception
  (add `AIPerceptionComponent.OnPerceptionUpdated` (`self.AIPerception`) (delegate `OnTargetSeen`)))

(event `self.ReceiveAnyDamage`
  (params (Damage :type "Float (single-precision)") (DamageType :type "DamageType Object Reference") (InstigatedBy :type "Controller Object Reference") (DamageCauser :type "Actor Object Reference"))
  ; Health and Death
  (if (not (`self.IsDead`))
    (set `self.Health` (- (`self.Health`) Damage))
    (`KismetSystemLibrary.PrintString` "tookdamage")
    (if (<= (`self.Health`) 0.0)
      (`self.Die`))))

(event `OnTargetSeen`
  (params (UpdatedActors :type "Array of Actor Object Reference (by ref)"))
  ; AI perception
  (for _array_element UpdatedActors
    (bind _asbp_player_character (cast `/Game/Variant_Platforming/Blueprints/BP_PlayerCharacter` _array_element))
    (set `self.PlayerRef` _asbp_player_character)
    (bind _asbp_enemy_aicontroller (cast `/Game/Enemy/BP_EnemyAIController` (`self.GetController`)))
    (`/Game/Enemy/BP_EnemyAIController.SetTarget` _asbp_enemy_aicontroller _asbp_player_character)))

(event `Die`
  (bind _mesh (`self.Mesh`))
  ; Health and Death
  (set `self.IsDead` true)
  (`PrimitiveComponent.SetSimulatePhysics` _mesh true)
  (`SkeletalMeshComponent.SetPhysicsBlendWeight` _mesh 10.0)
  (`PrimitiveComponent.SetCollisionEnabled` _mesh "QueryAndPhysics")
  (`KismetSystemLibrary.Delay` 1.4)
  (`self.K2_DestroyActor`))

(event `TryShootPlayer`
  (bind _enemygun (`self.EnemyGun`))
  (bind (_returnvalue_location _returnvalue_rotation) (`KismetMathLibrary.BreakTransform` (`SceneComponent.GetSocketTransform` _enemygun "Barrel" "RTS_World")))
  (if (`self.IsDead`)
    _
    (elif (`self.CanShoot`)
      (if (<= (`self.GetDistanceTo` (`self.PlayerRef`)) (`self.ShootingRange`))
        (if (>= (`KismetMathLibrary.Dot_VectorVector` (`self.GetActorForwardVector`) (`KismetMathLibrary.Normal` (- (`self.K2_GetActorLocation` (`self.PlayerRef`)) (`self.K2_GetActorLocation`)))) 0.4)
          (bind (_outhit _returnvalue) (`KismetSystemLibrary.LineTraceSingle` _returnvalue_location (+ (+ (* (`KismetMathLibrary.GetForwardVector` _returnvalue_rotation) (`self.ShootingRange`)) (`SceneComponent.K2_GetComponentLocation` _enemygun)) (* (* (`KismetMathLibrary.RandomUnitVector`) (- (`self.Accuracy`) 1.0)) (`self.SpreadMultiplier`))) "TraceTypeQuery1" false (`|MakeArray` self :!type "Actor Object Reference") "Persistent"))
          (if _returnvalue
            (`GameplayStatics.ApplyDamage` (`.HitActor` (`GameplayStatics.BreakHitResult` _outhit)) 10.0)
            (set `self.CanShoot` false)
            (`KismetSystemLibrary.Delay` (`self.FireRate`))
            (set `self.CanShoot` true)))))))

(fn `UserConstructionScript`)