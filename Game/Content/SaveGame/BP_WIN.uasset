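; BP_WIN is a win trigger that ends the game when the player character overlaps its box.
; On overlap it removes the ammo HUD, stops the custom game mode's timer, and shows the winning screen widget with a background fade.
; It then pauses the game, switches input to UI only and shows the mouse cursor.
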(event `self.Box.OnComponentBeginOverlap`
  (params (OverlappedComponent :type "PrimitiveComponent Object Reference") (OtherActor :type "Actor Object Reference") (OtherComp :type "PrimitiveComponent Object Reference") (OtherBodyIndex :type Integer) (bFromSweep :type Boolean) (SweepResult :type "HitResult Structure (by ref)"))
  (bind _returnvalue (`GameplayStatics.GetPlayerController` 0))
  (cast `/Game/Variant_Platforming/Blueprints/BP_PlayerCharacter` OtherActor)
  (bind _foundwidgets (`WidgetBlueprintLibrary.GetAllWidgetsOfClass` "/Game/Widgets/WBP_AMMOHUD.WBP_AMMOHUD_C"))
  (`Widget.RemoveFromParent` _foundwidgets)
  (bind _asbp_custom_game_mode (cast `/Game/SaveGame/BP_CustomGameMode` (`GameplayStatics.GetGameMode`)))
  (`/Game/SaveGame/BP_CustomGameMode.StopTimer` _asbp_custom_game_mode)
  (bind _returnvalue_2 (`|CreateWidget` "/Game/Widgets/WinningScreenWidget.WinningScreenWidget_C" (`GameplayStatics.GetPlayerController` 0)))
  (`UserWidget.AddToViewport` _returnvalue_2 0)
  (`/Game/Widgets/WinningScreenWidget.FadeBackground` _returnvalue_2)
  (`GameplayStatics.SetGamePaused` true)
  (`WidgetBlueprintLibrary.SetInputMode_UIOnlyEx` _returnvalue null)
  (set `PlayerController.bShowMouseCursor` true _returnvalue))

(fn `UserConstructionScript`)