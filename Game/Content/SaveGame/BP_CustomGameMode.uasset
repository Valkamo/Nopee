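; Game mode that runs a run timer and keeps a best time through BP_SaveGame.
; BeginPlay loads the "SAVE" slot into SessionBestTime, or creates it with a large sentinel time if absent.
; While TimerRunning is set, Tick accumulates elapsed time and splits it into minutes, seconds and milliseconds.
; StopTimer halts the clock, reloads the slot and passes the elapsed time to SaveBestTime.
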(event `self.ReceiveTick`
  (params (DeltaSeconds :type "Float (single-precision)"))
  ; Timer
  (if (`self.TimerRunning`)
    (set `self.ElapsedTime` (+ DeltaSeconds (`self.ElapsedTime`)))
    (set `self.Minutes` (`KismetMathLibrary.FFloor` (/ (`self.ElapsedTime`) 60.0)))
    (set `self.Seconds` (`KismetMathLibrary.FFloor` (mod (`self.ElapsedTime`) 60.0)))
    (set `self.Milliseconds` (`KismetMathLibrary.FFloor` (* (- (`self.ElapsedTime`) (`KismetMathLibrary.FFloor` (`self.ElapsedTime`))) 1000.0)))))

(event `self.ReceiveBeginPlay`
  ; CheckIfSaveGameExists
  (bind _returnvalue (`GameplayStatics.DoesSaveGameExist` "SAVE"))
  (if _returnvalue
    (bind _returnvalue_2 (`GameplayStatics.LoadGameFromSlot` "SAVE"))
    (bind _asbp_save_game (cast `/Game/SaveGame/BP_SaveGame` _returnvalue_2))
    (`/Game/SaveGame/BP_SaveGame.LoadBestTime` _asbp_save_game)
    (set `self.SessionBestTime` (`/Game/SaveGame/BP_SaveGame.SavedBestTime` _asbp_save_game))
    (else
      (bind _returnvalue_3 (`GameplayStatics.CreateSaveGameObject` "/Game/SaveGame/BP_SaveGame.BP_SaveGame_C"))
      (set `/Game/SaveGame/BP_SaveGame.SavedBestTime` 9999.0 _returnvalue_3)
      (`GameplayStatics.SaveGameToSlot` _returnvalue_3 "SAVE")
      (set `self.SessionBestTime` 9999.0))))

(event `StopTimer`
  ;[0 1 0.2292] Purpose:
  ;    - Stops the timer and calls BP_SaveGame to save the best time.
  ;
  ;  Logic:
  ;     Load Game from Slot ("BestTimeSlot") ✅
  ;     Cast to BP_SaveGame ✅
  ;     Call SaveBestTime (NewTime = ElapsedTime) ✅
  (set `self.TimerRunning` false)
  (bind _returnvalue (`GameplayStatics.LoadGameFromSlot` "SAVE"))
  (bind _asbp_save_game (cast `/Game/SaveGame/BP_SaveGame` _returnvalue))
  (`/Game/SaveGame/BP_SaveGame.SaveBestTime` _asbp_save_game (`self.ElapsedTime`))
  (`KismetSystemLibrary.PrintString` "\"Saving Best Time: \" + ElapsedTime"))

(fn `UserConstructionScript`
  (`parent.UserConstructionScript`))