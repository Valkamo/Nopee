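; BP_SaveGame is a save game object that tracks best and last run times, using 9999 as the no-record value.
; LoadBestTime returns its own SavedBestTime without using the loaded object, or saves a newly created object when no slot exists.
; SaveBestTime records each run time but writes itself to the "SAVE" slot only for a new best.
; ResetBestTime clears both times and saves.
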(fn `LoadBestTime`
  (returns (BestTimeOut :type "Float (double-precision)"))
  (bind _returnvalue (`GameplayStatics.DoesSaveGameExist` "SAVE"))
  (if _returnvalue
    (`GameplayStatics.LoadGameFromSlot` "SAVE")
    (`KismetSystemLibrary.PrintString` null "Save File Loaded Successfully!")
    (bind _output_get (set `self.Best Time Out` (`self.SavedBestTime`)))
    (else
      (bind _returnvalue_2 (`GameplayStatics.CreateSaveGameObject` "BP_SaveGame_C"))
      (set `self.SavedBestTime` 9999.0)
      (`GameplayStatics.SaveGameToSlot` _returnvalue_2 "SAVE")
      (set `self.Best Time Out` 9999.0)))
  (return _output_get))

(fn `ResetBestTime`
  (set `self.SavedBestTime` 9999.0)
  (set `self.LastRunTime` -1.0)
  (`GameplayStatics.SaveGameToSlot` self "SAVE")
  (`KismetSystemLibrary.PrintString` null "Best Time Reset to No Record!"))

(fn `SaveBestTime`
  (params (NewTime :type "Float (double-precision)"))
  (set `self.LastRunTime` NewTime)
  (if (or (== (`self.SavedBestTime`) 9999.0) (< NewTime (`self.SavedBestTime`)))
    (set `self.SavedBestTime` NewTime)
    (`GameplayStatics.SaveGameToSlot` self "SAVE")
    (`KismetSystemLibrary.PrintString` null "save" true true (struct :`G` 1.0 :`B` 0.229244 :`A` 1.0) 5.0)))