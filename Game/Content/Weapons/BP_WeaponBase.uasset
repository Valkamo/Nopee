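; Base weapon Blueprint with shotgun behavior: pellet-spread hitscan fire, pump animations, ammo tracking and shell-by-shell reload.
; FireWeapon spends one round, plays camera shake and muzzle flash, then runs randomized camera line traces that damage hit actors.
; CanFire gates shots and re-arms after the FireRate delay only when a trace hits, or when reloading finishes.
; Reload tilts the mesh, recursively loads shells on a delay, then restores the BeginPlay transform.
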(event `self.ReceiveBeginPlay`
  ; Set baserotation of the weapon
  (set `self.BaseRotation` (`SceneComponent.RelativeRotation` (`self.WeaponMesh`)))
  (set `self.BaseLocation` (`SceneComponent.RelativeLocation` (`self.WeaponMesh`)))
  (bind _returnvalue (`GameplayStatics.GetActorOfClass` "/Game/Variant_Platforming/Blueprints/BP_PlayerCharacter.BP_PlayerCharacter_C"))
  (set `self.PlayerRef` _returnvalue))

(event `FireWeapon`
  (bind _spread (`self.Spread`))
  (bind _playercameramanager (`PlayerController.PlayerCameraManager` (`GameplayStatics.GetPlayerController` 0)))
  (bind _returnvalue (`PlayerCameraManager.GetCameraLocation` _playercameramanager))
  (if (`self.CanFire`)
    (set `self.CanFire` false)
    (if (`self.IsReloading`)
      _
      (elif (not (<= (`self.CurrentAmmoInMag`) 0))
        (`PlayerController.ClientStartCameraShake` :`self` (`GameplayStatics.GetPlayerController` 0) :`Shake` "/Game/Weapons/CS_ShotgunFire.CS_ShotgunFire_C")
        (`NiagaraFunctionLibrary.SpawnSystemAttached` "/Game/Effects/Niagara/ShotGunMuzzleFlash.ShotGunMuzzleFlash" (`self.WeaponMesh`) "MuzzleFlash" (0.0 0.0 0.0) (struct) "SnapToTarget" true)
        (bind _result (`/Engine/EditorBlueprintResources/StandardMacros.DecrementInt` (`self.CurrentAmmoInMag`))
          (:`  `
            (set `self.CurrentAmmoInMag` _result)
            (for _ (range 11)
              (bind (_outhit _returnvalue_2) (`KismetSystemLibrary.LineTraceSingle` _returnvalue (+ _returnvalue (* (`KismetMathLibrary.GetForwardVector` (`PlayerCameraManager.GetCameraRotation` _playercameramanager)) (`self.Range`)) (`KismetMathLibrary.MakeVector` (`KismetMathLibrary.RandomFloatInRange` (* _spread -1.0) _spread) (`KismetMathLibrary.RandomFloatInRange` (* _spread -1.0) _spread) (`KismetMathLibrary.RandomFloatInRange` (* _spread -1.0) _spread))) "TraceTypeQuery1" false (`|MakeArray` (`self.PlayerRef`) :!type "Actor Object Reference") "ForOneFrame"))
              (if _returnvalue_2
                ; Pump
                (`SkeletalMeshComponent.PlayAnimation` (`self.WeaponMesh`) "/Game/package/Animation/Anim_fire.Anim_fire" false)
                (`GameplayStatics.ApplyDamage` (`.HitActor` (`GameplayStatics.BreakHitResult` _outhit)) (`self.Damage`))
                (`KismetSystemLibrary.Delay` (`self.FireRate`))
                ; UnPump
                (`SkeletalMeshComponent.PlayAnimation` (`self.WeaponMesh`) "/Game/package/Animation/Anim_fireReverse.Anim_fireReverse" false)
                (set `self.CanFire` true)
                (else
                  (`SkeletalMeshComponent.PlayAnimation` (`self.WeaponMesh`) "/Game/package/Animation/Anim_fire.Anim_fire" false))))))))))

(event `ReloadStart`
  ; Start reload make the reload animation
  (if (not (`self.IsReloading`))
    (set `self.CanFire` false)
    (`SceneComponent.K2_SetRelativeLocationAndRotation` (`self.WeaponMesh`) (40.0 10.0 -10.0) (struct :`Yaw` 240.0 :`Roll` -40.0) false false)
    (`self.ReloadLoop`)))

(event `ReloadLoop`
  ; Reload
  (set `self.CanFire` false)
  (if (or (>= (`self.CurrentAmmoInMag`) (`self.MagazineSize`)) (<= (`self.SpareAmmo`) 0))
    (`self.ReloadFinished`)
    (else
      (`SkeletalMeshComponent.PlayAnimation` (`self.WeaponMesh`) "/Game/package/Animation/Anim_reload.Anim_reload" false)
      (`KismetSystemLibrary.Delay` (`self.FireRate`))
      (if (or (>= (`self.CurrentAmmoInMag`) (`self.MagazineSize`)) (<= (`self.SpareAmmo`) 0))
        (`self.ReloadFinished`)
        (else
          (`/Engine/EditorBlueprintResources/StandardMacros.IncrementInt` (`self.CurrentAmmoInMag`)
            (:`  `
              (`/Engine/EditorBlueprintResources/StandardMacros.DecrementInt` (`self.SpareAmmo`)
                (:`  `
                  (`self.ReloadLoop`))))))))))

(event `ReloadFinished`
  ; Set weapon to fire again and set weapon to default position after a reload
  (set `self.CanFire` false)
  (`SceneComponent.K2_SetRelativeLocationAndRotation` (`self.WeaponMesh`) (`self.BaseLocation`) (`self.BaseRotation`) false false)
  (set `self.IsReloading` false)
  (set `self.CanFire` true))

(fn `UserConstructionScript`)